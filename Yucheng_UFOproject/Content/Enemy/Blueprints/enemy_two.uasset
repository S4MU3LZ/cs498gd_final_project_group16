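; Enemy actor that fires Magic_ball projectiles in a repeating three-way volley.
; From BeginPlay it loops on a one-second delay, calling ShootThreeDirections to spawn balls at the front, left-front and right-front components.
; Only the front ball has its velocity set, along world X rather than the spawn facing.
; QuickShootFront repeats the front shot alone but is not called in this graph.
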(event EventBeginPlay
  ;[1 1 1] make projectile
  (Utilities|FlowControl|Delay 1.0 :!label _label)
  (CallFunction|ShootThreeDirections)
  (goto _label))

(event Collision|EventActorBeginOverlap
  (params (OtherActor :type Actor%20Object%20Reference)))

(event EventTick
  (params (DeltaSeconds :type Float%20%28single-precision%29)))

(fn ConstructionScript)

(fn QuickShootFront
  (bind _magicballfront (Variables|Default|GetMagicBallFront))
  (bind _returnvalue (Game|SpawnActorfromClass "/Game/Enemy/Blueprints/magic_ball.magic_ball_C" (Math|Transform|MakeTransform (Transformation|GetWorldLocation _magicballfront) (Transformation|GetWorldRotation _magicballfront) "1,1,1") "Undefined" 0 0))
  (Class|PrimitiveComponent|SetAllPhysicsLinearVelocity (Variables|/Game/Enemy/Blueprints/magic_ball.magic_ball_C|GetSphere _returnvalue) "100.000000, 0, 0" false))

(fn ShootThreeDirections
  (bind _magicballfront (Variables|Default|GetMagicBallFront))
  (bind _returnvalue (Game|SpawnActorfromClass "/Game/Enemy/Blueprints/magic_ball.magic_ball_C" (Math|Transform|MakeTransform (Transformation|GetWorldLocation _magicballfront) (Transformation|GetWorldRotation _magicballfront) "1,1,1") "Undefined" 0 0))
  (Class|PrimitiveComponent|SetAllPhysicsLinearVelocity (Variables|/Game/Enemy/Blueprints/magic_ball.magic_ball_C|GetSphere _returnvalue) "100.000000, 0, 0" false)
  (Game|SpawnActorfromClass "/Game/Enemy/Blueprints/magic_ball.magic_ball_C" (Transformation|GetWorldTransform (Variables|Default|GetMagicBallLeftFront)) "Undefined" 0 0)
  (Game|SpawnActorfromClass "/Game/Enemy/Blueprints/magic_ball.magic_ball_C" (Transformation|GetWorldTransform (Variables|Default|GetMagicBallRightFront)) "Undefined" 0 0))