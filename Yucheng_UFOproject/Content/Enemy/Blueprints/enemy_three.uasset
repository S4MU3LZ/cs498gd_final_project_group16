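; Enemy actor that lobs a physics-driven bomb from its front muzzle once a second, looping from BeginPlay.
; ArcBomb spawns the bomb and launches it with a suggested arc velocity, scaled up threefold, toward one of three aim points.
; SetBombEndLocation picks that point with two separate random rolls, so the odds are uneven.
; QuickShootFront, a straight Magic_ball shot along world X, is defined but never called here.
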(event EventBeginPlay
  ;[1 1 1] make projectile
  (Utilities|FlowControl|Delay 1.0 :!label _label)
  (CallFunction|ArcBomb)
  (goto _label))

(event Collision|EventActorBeginOverlap
  (params (OtherActor :type Actor%20Object%20Reference)))

(event EventTick
  (params (DeltaSeconds :type Float%20%28single-precision%29)))

(fn ConstructionScript)

(fn QuickShootFront
  (bind _magicballfront (Variables|Default|GetMagicBallFront))
  (bind _returnvalue (Game|SpawnActorfromClass "/Game/Enemy/Blueprints/magic_ball.magic_ball_C" (Math|Transform|MakeTransform (Transformation|GetWorldLocation _magicballfront) (Transformation|GetWorldRotation _magicballfront) "1,1,1") "Undefined" 0 0))
  (Class|PrimitiveComponent|SetAllPhysicsLinearVelocity (Variables|/Game/Enemy/Blueprints/magic_ball.magic_ball_C|GetSphere _returnvalue) "100.000000, 0, 0" false))

(fn ArcBomb
  (bind _magicballfront (Variables|Default|GetMagicBallFront))
  (bind _returnvalue (Game|SpawnActorfromClass "/Game/Enemy/Blueprints/bomb.bomb_C" (Transformation|GetWorldTransform _magicballfront) "Undefined" 0 0))
  (CallFunction|SetBombEndLocation)
  (bind _outlaunchvelocity (Game|SuggestProjectileVelocityCustomArc (Transformation|GetWorldLocation _magicballfront) (Variables|Default|Getend_bomb_position) 0.0 0.5))
  (Physics|SetPhysicsLinearVelocity (Variables|/Game/Enemy/Blueprints/bomb.bomb_C|GetBomb _returnvalue) (* _outlaunchvelocity 3.0) false "None"))

(fn SetBombEndLocation
  (bind _returnvalue (Math|Random|RandomIntegerinRange 0 2))
  (if (== _returnvalue 0)
    (Variables|Default|Setend_bomb_position (Transformation|GetWorldLocation (Variables|Default|GetBombAim1)))
    (elif (== _returnvalue 1)
      (Variables|Default|Setend_bomb_position (Transformation|GetWorldLocation (Variables|Default|GetBombAim2)))
      (else
        (Variables|Default|Setend_bomb_position (Transformation|GetWorldLocation (Variables|Default|GetBombAim3)))))))